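; SurfaceBuilder is an actor Blueprint that builds a vertex-colored surface mesh at runtime from coordinate data stored in the platform user directory.
; On BeginPlay it checks for the coordinates file and creates a default one if that check fails.
; GetNodes then supplies vertices, triangles and colors to a ProceduralMesh section, which receives the VertexColor material.
; The construction script is empty, so all generation happens at BeginPlay.
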(event EventBeginPlay
  (bind _returnvalue (Class|SurfaceNodeUtils|CheckCoordinatesFile (Class|KismetSystemLibrary|GetPlatformUserDir)))
  (if _returnvalue
    _
    (else
      (Class|SurfaceNodeUtils|CreateDefaultCoordintatesFile (Class|KismetSystemLibrary|GetPlatformUserDir))))
  (bind (_coordinates _triangles _vertexcolors) (Class|SurfaceNodeUtils|GetNodes (Class|KismetSystemLibrary|GetPlatformUserDir)))
  (Class|ProceduralMeshComponent|CreateMeshSectionLinearColor (Variables|Default|GetProceduralMesh) 0 _coordinates _triangles 0 0 0 0 0 _vertexcolors 0 false false)
  (Rendering|Material|SetMaterial (Variables|Default|GetProceduralMesh) 0 "/Game/Baikal4/Blueprints/VertexColor.VertexColor"))

(event Collision|EventActorBeginOverlap
  (params (OtherActor :type Actor%20Object%20Reference)))

(event EventTick
  (params (DeltaSeconds :type Float%20%28single-precision%29)))

(fn ConstructionScript)