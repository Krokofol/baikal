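; Actor that builds a procedural, vertex-colored terrain mesh from a coordinates file in the user directory and lets the player rotate and scale it.
; On BeginPlay it creates a default file if missing, loads the node grid, downsamples it to a node limit and builds a colliding mesh scaled to a maximum size.
; Enhanced Input drives stepped scaling and per-tick yaw and clamped-pitch rotation, with events to add or remove mapping contexts.
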(event Custom|RemoveMappingContexts
  (bind _returnvalue (Game|GetPlayerController 0))
  (bind _returnvalue_2 (PlayerController|LocalPlayerSubsystems|GetEnhancedInputLocalPlayerSubsystem _returnvalue))
  (if (.ReturnValue (Class|EnhancedInputSubsystemInterface|HasMappingContext _returnvalue_2 "/Game/Baikal4/Input/IMC_Rotation.IMC_Rotation"))
    (Input|RemoveMappingContext _returnvalue_2 "/Game/Baikal4/Input/IMC_Rotation.IMC_Rotation" "(bIgnoreAllPressedKeysUntilRelease=True,bForceImmediately=False)"))
  (if (.ReturnValue (Class|EnhancedInputSubsystemInterface|HasMappingContext _returnvalue_2 "/Game/Baikal4/Input/IMC_Scale.IMC_Scale"))
    (Input|RemoveMappingContext _returnvalue_2 "/Game/Baikal4/Input/IMC_Scale.IMC_Scale" "(bIgnoreAllPressedKeysUntilRelease=True,bForceImmediately=False)")))

(event Custom|AddMappingContext
  (params (InputMappingContext :type Input%20Mapping%20Context%20Object%20Reference))
  (Input|AddMappingContext (PlayerController|LocalPlayerSubsystems|GetEnhancedInputLocalPlayerSubsystem (Game|GetPlayerController 0)) InputMappingContext 0 "(bIgnoreAllPressedKeysUntilRelease=True,bForceImmediately=False)"))

(event Input|EnhancedActionEvents|EnhancedInputActionIA_Scale
  (params (ActionValue :type Float%20%28double-precision%29) (ElapsedSeconds :type Float%20%28double-precision%29) (TriggeredSeconds :type Float%20%28double-precision%29) (InputAction :type Input%20Action%20Object%20Reference :default "/Game/Baikal4/Input/Actions/IA_Scale.IA_Scale"))
  (:Started
    (CallFunction|Scale ActionValue)))

(event EventBeginPlay
  (Input|EnableInput (Game|GetPlayerController 0))
  (CallFunction|GenerateSurface))

(event Collision|EventActorBeginOverlap
  (params (OtherActor :type Actor%20Object%20Reference)))

(event EventTick
  (params (DeltaSeconds :type Float%20%28single-precision%29))
  (CallFunction|Rotate DeltaSeconds))

(fn ConstructionScript)

(fn GenerateSurface
  (bind _returnvalue (Class|SurfaceNodeUtils|CheckCoordinatesFile (Class|KismetSystemLibrary|GetPlatformUserDir)))
  (if _returnvalue
    _
    (else
      (Class|SurfaceNodeUtils|CreateDefaultCoordintatesFile (Class|KismetSystemLibrary|GetPlatformUserDir))))
  (bind (_coordinates _nodescountx _nodescounty) (Class|SurfaceNodeUtils|GetNodes (Class|KismetSystemLibrary|GetPlatformUserDir) (Variables|Consts|GetHorizontal%20Scale)))
  (Variables|Surface|SetNodes%20Count%20X _nodescountx)
  (Variables|Surface|SetNodes%20Count%20Y _nodescounty)
  (Variables|Surface|SetNodes _coordinates)
  (bind (_nodes_count_x _nodes_count_y _nodes) (CallFunction|GenerateScaledSurface 0 (- (* (Variables|Surface|GetNodes%20Count%20X) (Variables|Surface|GetNodes%20Count%20Y)) 1) 1000))
  (bind _returnvalue_2 (Class|SurfaceNodeUtils|ColorVertexes _nodes))
  (bind _triangles (Class|SurfaceNodeUtils|GenerateTriangles _nodes_count_x _nodes_count_y))
  (Class|ProceduralMeshComponent|CreateMeshSectionLinearColor (Variables|Default|GetProceduralMesh) 0 _nodes _triangles 0 0 0 0 0 _returnvalue_2 0 true false)
  (Rendering|Material|SetMaterial (Variables|Default|GetProceduralMesh) 0 "/Game/Baikal4/Blueprints/SurfaceBuilder/VertexColor.VertexColor")
  (bind _scale (CallFunction|CalculateAxisScale 2e+02 (Variables|Surface|GetNodes%20Count%20X) (Variables|Surface|GetNodes%20Count%20Y)))
  (Transformation|SetActorScale3D (Math|Vector|MakeVector _scale _scale _scale)))

(fn CalculateAxisScale
  (params (Max%20Size :type Float%20%28double-precision%29) (Nodes%20Count%20X :type Integer) (Nodes%20Count%20Y :type Integer))
  (return (/ Max%20Size (* (Math|Float|Max(Float) (Math|Conversions|ToFloat(Integer) Nodes%20Count%20X) (Math|Conversions|ToFloat(Integer) Nodes%20Count%20Y)) (Variables|Consts|GetHorizontal%20Scale)))))

(fn GenerateScaledSurface
  (params (Node1 :type Integer) (Node2 :type Integer) (Max%20Nodes%20Per%202%20Meters :type Integer))
  (bind _nodes_count_x (Variables|Surface|GetNodes%20Count%20X))
  (bind _nodes_count_y (Variables|Surface|GetNodes%20Count%20Y))
  (if false
    (return (Variables|Surface|GetNodes%20Count%20X) (Variables|Surface|GetNodes%20Count%20Y) (Variables|Surface|GetNodes))
    (else
      (bind (_node_number_x _node_number_y) (CallFunction|GetNode'sXY Node1 _nodes_count_x _nodes_count_y))
      (LocalVariables|SetX1 _node_number_x)
      (LocalVariables|SetY1 _node_number_y)
      (bind (_node_number_x_2 _node_number_y_2) (CallFunction|GetNode'sXY Node2 _nodes_count_x _nodes_count_y))
      (bind _output_get (LocalVariables|SetX2 _node_number_x_2))
      (bind _output_get_2 (LocalVariables|SetY2 _node_number_y_2))
      (bind _output_get_3 (LocalVariables|SetDX (Math|Integer|Absolute(Integer) (- _output_get (LocalVariables|GetX1)))))
      (bind _output_get_4 (LocalVariables|SetDY (Math|Integer|Absolute(Integer) (- _output_get_2 (LocalVariables|GetY1)))))
      (bind _returnvalue (Class|SurfaceNodeUtils|TakeEach (LocalVariables|GetX1) (LocalVariables|GetY1) (LocalVariables|GetX2) (LocalVariables|GetY2) (Variables|Surface|GetNodes) (Math|Float|Ceil (/ (Math|Conversions|ToFloat(Integer) (Math|Integer|Max(Integer) _output_get_3 _output_get_4)) (Math|Conversions|ToFloat(Integer) Max%20Nodes%20Per%202%20Meters))) (Variables|Surface|GetNodes%20Count%20X) (Variables|Surface|GetNodes%20Count%20Y)))
      (return (+ (/ _output_get_3 (Math|Float|Ceil (/ (Math|Conversions|ToFloat(Integer) (Math|Integer|Max(Integer) _output_get_3 _output_get_4)) (Math|Conversions|ToFloat(Integer) Max%20Nodes%20Per%202%20Meters)))) (Class|KismetMathLibrary|SignOfInteger (+ (Math|Integer|%(Integer) _output_get_3 (Math|Float|Ceil (/ (Math|Conversions|ToFloat(Integer) (Math|Integer|Max(Integer) _output_get_3 _output_get_4)) (Math|Conversions|ToFloat(Integer) Max%20Nodes%20Per%202%20Meters)))) 1))) (+ (/ _output_get_4 (Math|Float|Ceil (/ (Math|Conversions|ToFloat(Integer) (Math|Integer|Max(Integer) _output_get_3 _output_get_4)) (Math|Conversions|ToFloat(Integer) Max%20Nodes%20Per%202%20Meters)))) (Class|KismetMathLibrary|SignOfInteger (+ (Math|Integer|%(Integer) _output_get_4 (Math|Float|Ceil (/ (Math|Conversions|ToFloat(Integer) (Math|Integer|Max(Integer) _output_get_3 _output_get_4)) (Math|Conversions|ToFloat(Integer) Max%20Nodes%20Per%202%20Meters)))) 1))) _returnvalue))))

(fn GetNode'sXY
  (params (Node%20Number :type Integer) (Nodes%20Count%20X :type Integer) (Nodes%20Count%20Y :type Integer))
  (return (Math|Integer|%(Integer) Node%20Number Nodes%20Count%20X) (/ Node%20Number Nodes%20Count%20X)))

(fn Scale
  (params (value :type Float%20%28double-precision%29))
  (bind _proceduralmesh (Variables|Default|GetProceduralMesh))
  (bind _returnvalue (Transformation|GetWorldScale _proceduralmesh))
  (if (> value 0.0)
    (LocalVariables|SetScaleValue 1.25)
    (else
      (LocalVariables|SetScaleValue 0.8)))
  (Transformation|SetWorldScale3D _proceduralmesh (Math|Vector|MakeVector (* (.x _returnvalue) (LocalVariables|GetScaleValue)) (* (.y _returnvalue) (LocalVariables|GetScaleValue)) (* (.z _returnvalue) (LocalVariables|GetScaleValue)))))

(fn Rotate
  (params (delta%20time :type Float%20%28double-precision%29))
  (bind _returnvalue (Input|EnhancedActionValues|GetIA_Rotation))
  (bind _fullspeed (LocalVariables|GetFullSpeed))
  (bind _proceduralmesh (Variables|Default|GetProceduralMesh))
  (bind _returnvalue_2 (Transformation|GetWorldRotation _proceduralmesh))
  (bind _returnvalue_3 (* delta%20time _fullspeed))
  (LocalVariables|SetSpeedX (* _returnvalue_3 (.x _returnvalue)))
  (LocalVariables|SetSpeedY (* _returnvalue_3 (.y _returnvalue)))
  (Transformation|SetWorldRotation _proceduralmesh (Math|Rotator|MakeRotator (.roll _returnvalue_2) (Math|Float|Min(Float) (Math|Float|Max(Float) (+ (.pitch _returnvalue_2) (LocalVariables|GetSpeedY)) -3e+01) 3e+01) (+ (.yaw _returnvalue_2) (LocalVariables|GetSpeedX))) false false))